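; Survival Blueprint that continuously spawns Basic_Zeacon_survival AI pawns.
; BeginPlay calls GAMESTART, which starts a looping timer with the Speed variable as its interval.
; Each tick of the timer gathers all Zceaconspawner actors and spawns one pawn at the location of a randomly chosen spawner.
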(event `self.ReceiveBeginPlay`
  (`self.GAME START`))

(event `GAME START`
  (`KismetSystemLibrary.K2_SetTimerDelegate` (delegate `Spawn Zceacon`) (`self.Speed`) true))

(event `Spawn Zceacon`
  (bind _outactors (`GameplayStatics.GetAllActorsOfClass` "/Game/FirstPersonBP/Blueprints/zceaconspawner.zceaconspawner_C"))
  (`AIBlueprintHelperLibrary.SpawnAIFromClass` "/Game/FirstPersonBP/Blueprints/Basic_Zeacon_survival.Basic_Zeacon_survival_C" null (`self.K2_GetActorLocation` (`|GetArrayItem` _outactors (`KismetMathLibrary.RandomInteger` (`KismetArrayLibrary.Array_Length` _outactors))))))

(fn `UserConstructionScript`
  (`parent.UserConstructionScript`))