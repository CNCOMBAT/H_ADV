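; Survival mode wave spawner that sends AI enemies out at random Zceaconspawner points with escalating pressure.
; A self-repeating Spawn loop creates a Basic_Zeacon_survival plus chance-based Teacon_survival and Spreecan, paced by the Speed delay.
; A recurring Speedup timer shortens that delay and spawns an Indicator until Speed hits its floor.
; At the floor, each Speedup instead spawns random Teacon and Spreecan bursts and re-triggers GAMESTART.
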(event `self.ReceiveBeginPlay`
  (`self.GAME START`)
  (`KismetSystemLibrary.Delay` 20.0)
  (`self.speedup`))

(event `GAME START`
  (`self.spawn`))

(event `spawn`
  (bind _outactors (`GameplayStatics.GetAllActorsOfClass` "/Game/FirstPersonBP/Blueprints/zceaconspawner.zceaconspawner_C"))
  (bind _returnvalue (`self.K2_GetActorLocation` (`|GetArrayItem` _outactors (`KismetMathLibrary.RandomInteger` (`KismetArrayLibrary.Array_Length` _outactors)))))
  (`AIBlueprintHelperLibrary.SpawnAIFromClass` "/Game/FirstPersonBP/Blueprints/Basic_Zeacon_survival.Basic_Zeacon_survival_C" null _returnvalue)
  (`|ExecutionSequence`
    (:`then_0`
      (if (== (`KismetMathLibrary.RandomIntegerInRange` 0 5) 0)
        (`AIBlueprintHelperLibrary.SpawnAIFromClass` "/Game/FirstPersonBP/Blueprints/Teacon_survival.Teacon_survival_C" null _returnvalue)))
    (:`then_1`
      (if (== (`KismetMathLibrary.RandomIntegerInRange` 0 3) 0)
        (`AIBlueprintHelperLibrary.SpawnAIFromClass` "/Game/FirstPersonBP/Blueprints/Spreecan.Spreecan_C" null _returnvalue)))
    (:`then_2`
      (`KismetSystemLibrary.Delay` (`self.Speed`))
      (`self.spawn`))))

(event `speedup`
  (bind _speed (`self.Speed`))
  (`|ExecutionSequence`
    (:`then_0`
      (set `self.Speed` (- _speed 0.25))
      (if (<= _speed 0.25)
        (set `self.Speed` 0.25)
        (`|ExecutionSequence`
          (:`then_0`
            (for _ (range 2 (+ (`KismetMathLibrary.RandomIntegerInRange` 0 4) 1))
              (bind _returnvalue (`self.K2_GetActorLocation` (`|GetArrayItem` (stale `spawn` _outactors) (`KismetMathLibrary.RandomInteger` (`KismetArrayLibrary.Array_Length` (stale `spawn` _outactors))))))
              (`AIBlueprintHelperLibrary.SpawnAIFromClass` "/Game/FirstPersonBP/Blueprints/Teacon_survival.Teacon_survival_C" null _returnvalue))
            (for _ (range (+ (`KismetMathLibrary.RandomIntegerInRange` 3 10) 1))
              (`AIBlueprintHelperLibrary.SpawnAIFromClass` "/Game/FirstPersonBP/Blueprints/Spreecan.Spreecan_C" null _returnvalue)))
          (:`then_1`
            (`KismetSystemLibrary.Delay` (`self.Speed`))
            (`self.GAME START`)))
        (else
          (`|SpawnActorFromClass` "/Game/FirstPersonBP/Blueprints/indicator.indicator_C" (`KismetMathLibrary.MakeTransform` (0.0 0.0 1000.0)) "Undefined" "OverrideRootScale" null null)
          (`KismetSystemLibrary.PrintString` (`KismetStringLibrary.Conv_DoubleToString` (`self.Speed`))))))
    (:`then_1`
      (`KismetSystemLibrary.Delay` (`KismetMathLibrary.RandomFloatInRange` 17.0 22.0))
      (`self.speedup`))))

(event `spawnpart`)

(fn `UserConstructionScript`
  (`parent.UserConstructionScript`))