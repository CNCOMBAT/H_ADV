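; SurvivalStateFix tracks how long the player has survived and animates a timed "start anew" transition value.
; A looping one-second timer started on BeginPlay increments seconds and rolls them over into minutes.
; The startnew event sets flags for three seconds, during which Tick interpolates StartingANew toward one, then flips them so it eases back to zero.
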(event `self.ReceiveTick`
  (params (DeltaSeconds :type "Float (single-precision)"))
  (`|ExecutionSequence`
    (:`then_0`
      (if (`self.change`)
        (set `self.starting a new` (`KismetMathLibrary.FInterpTo` (`self.starting a new`) 0.0 (`GameplayStatics.GetWorldDeltaSeconds`) 5.0))))
    (:`then_1`
      (if (and (`self.startyeet`) (not (`self.change`)))
        (set `self.starting a new` (`KismetMathLibrary.FInterpTo` (`self.starting a new`) 1.0 (`GameplayStatics.GetWorldDeltaSeconds`) 6.0))))))

(event `start new`
  (set `self.change` false)
  (set `self.startyeet` true)
  (`KismetSystemLibrary.Delay` 3.0)
  (set `self.startyeet` false)
  (set `self.change` true))

(event `self.ReceiveBeginPlay`
  (`KismetSystemLibrary.K2_SetTimerDelegate` (delegate `time reduction`) 1.0 true))

(event `time reduction`
  (bind _time_survived (`self.time survived`))
  (if (== _time_survived 59.0)
    (set `self.time survived` 0.0)
    (set `self.min survived` (+ (`self.min survived`) 1.0))
    (else
      (set `self.time survived` (+ _time_survived 1.0)))))

(fn `UserConstructionScript`)